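; Monster enemy that chases the player seen through PawnSensing and kills them on CatchZone overlap.
; Overlapping a hide locker drops the chase into looping random navmesh patrol, re-enabling sight after a delay.
; A timer, when sight is enabled but no chase is active, teleports it to the BP_EnemySpawn nearest the player.
; Stun and WakeUp events halt and resume it, and transform events swap human and monster meshes.
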(event OnSeePawn(PawnSensing)
  (params (Pawn :type Pawn%20Object%20Reference))
  ;[1 1 1] Chase player
  (Collision|SetCollisionEnabled (Variables|Default|GetCatchZone) "QueryOnly")
  (bind _asbp_third_person_character (Utilities|Casting|CastToBP_ThirdPersonCharacter Pawn))
  (if (Variables|Default|GetCanSeePlayer)
    (Variables|Default|SetChasingPlayer true)
    (Variables|/Script/Engine.CharacterMovementComponent|SetMaxWalkSpeed (Variables|Character|GetCharacterMovement) 2e+02)
    (Components|Timeline|SetPlayRate (Variables|Character|GetMesh) 3e+01)
    (CallFunction|Playgrowlsound)
    (Development|PrintString "Monster chase")
    (AI|AIMoveTo self "0, 0, 0" _asbp_third_person_character 5.0 false)))

(event OnComponentHit(Mesh)
  (params (HitComponent :type Primitive%20Component%20Object%20Reference) (OtherActor :type Actor%20Object%20Reference) (OtherComp :type Primitive%20Component%20Object%20Reference) (NormalImpulse :type Vector :default "0, 0, 0") (Hit :type Hit%20Result%20Structure%20%28by%20ref%29))
  ;[1 1 1] Catch player
)

(event OnComponentBeginOverlap(CatchZone)
  (params (OverlappedComponent :type Primitive%20Component%20Object%20Reference) (OtherActor :type Actor%20Object%20Reference) (OtherComp :type Primitive%20Component%20Object%20Reference) (OtherBodyIndex :type Integer) (bFromSweep :type Boolean) (SweepResult :type Hit%20Result%20Structure%20%28by%20ref%29))
  ;[1 1 1] Catch player
  (if (== (Utilities|GetClass OtherActor) "/Game/ThirdPerson/PhongBP/Assets/BP_HideLocker.BP_HideLocker_C")
    (CallFunction|LostSight)
    (else
      (Utilities|Casting|CastToBP_ThirdPersonCharacter OtherActor)
      (if (Variables|Default|GetChasingPlayer)
        (Development|PrintString "Catch player")
        (bind _asbp_third_person_character (Utilities|Casting|CastToBP_ThirdPersonCharacter OtherActor))
        (Default|PlayerDeath _asbp_third_person_character)))))

(event OnComponentHit(CapsuleComponent)
  (params (HitComponent :type Primitive%20Component%20Object%20Reference) (OtherActor :type Actor%20Object%20Reference) (OtherComp :type Primitive%20Component%20Object%20Reference) (NormalImpulse :type Vector :default "0, 0, 0") (Hit :type Hit%20Result%20Structure%20%28by%20ref%29))
  ;[1 1 1] Catch player
)

(event Custom|LostSight
  ;[1 1 1] Stun and lost sight
  (Variables|Default|SetCanSeePlayer false)
  (Variables|Default|SetChasingPlayer false)
  (Development|PrintString "Lost sight")
  (CallFunction|Patrol))

(event Custom|TPCheck
  ;[1 1 1] TP logic
  (Utilities|Time|SetTimerbyEvent (delegate Custom|TPCheck) 2.5 true)
  (if (not (Variables|Default|GetChasingPlayer))
    (if (Variables|Default|GetCanSeePlayer)
      (CallFunction|Teleport)
      (Development|PrintString "TP"))))

(event Custom|Teleport
  ;[1 1 1] TP logic
  (Audio|PlaySoundatLocation "/Game/Audio/shadow_tp_Cue.shadow_tp_Cue" (Transformation|GetActorLocation) "0, 0, 0" 1.0 1.0 0.0 0 0 0 0)
  (bind _outactors (Actor|GetAllActorsOfClass "/Game/Enemy/BP_EnemySpawn.BP_EnemySpawn_C"))
  (for _array_element _outactors
    (if (< (Math|Vector|Distance(Vector) (Transformation|GetActorLocation _array_element) (Transformation|GetActorLocation (Game|GetPlayerCharacter 0))) (Variables|Default|GetClosestDistance))
      (Variables|Default|SetClosestDistance (Math|Vector|Distance(Vector) (Transformation|GetActorLocation _array_element) (Transformation|GetActorLocation (Game|GetPlayerCharacter 0))))
      (Variables|Default|SetBestSpawnPoint (Transformation|GetActorLocation _array_element))))
  (Transformation|SetActorLocation (Variables|Default|GetBestSpawnPoint) false false)
  (Variables|Default|SetBestSpawnPoint "0.000000,0.000000,20.000000")
  (Variables|Default|SetClosestDistance 1e+04))

(event Custom|Stun
  ;[1 1 1] Stun and lost sight
  (Pawn|Components|CharacterMovement|DisableMovement (Variables|Character|GetCharacterMovement))
  (Variables|Default|SetCanSeePlayer false)
  (Variables|Default|SetChasingPlayer false)
  (Development|PrintString "Monster stun")
  (Audio|Components|Audio|Stop (Variables|Character|GetMesh))
  (CallFunction|Speak))

(event Custom|WakeUp
  ;[1 1 1] Stun and lost sight
  (Pawn|Components|CharacterMovement|SetMovementMode (Variables|Character|GetCharacterMovement) "MOVE_Walking" 0)
  (Development|PrintString "Monster wake up")
  (CallFunction|LostSight)
  (Components|Animation|PlayAnimation (Variables|Character|GetMesh) "/Game/Enemy/monster1/monster_Anim.monster_Anim" true))

(event Custom|Patrol
  ;[1 1 1] random patrol when game start
  (Variables|/Script/Engine.CharacterMovementComponent|SetMaxWalkSpeed (Variables|Character|GetCharacterMovement) 1e+02)
  (Components|Timeline|SetPlayRate (Variables|Character|GetMesh) 3.0)
  (Development|PrintString "Monster patrol")
  (bind _randomlocation (Class|NavigationSystemV1|GetRandomLocationinNavigableRadius (Transformation|GetActorLocation) 5e+02 0 0 :!label _label))
  (AI|AIMoveTo self _randomlocation 0 5.0 false
    (:then
      (Utilities|FlowControl|Delay 1e+01)
      (Variables|Default|SetCanSeePlayer true))
    (:OnSuccess
      (goto _label))
    (:OnFail
      (goto _label))))

(event Custom|Transform%20to%20human
  ;[1 1 1] Transform and display message
  (Components|SkeletalMesh|SetSkeletalMeshAsset (Variables|Character|GetMesh) "/Game/Characters/Mannequin_UE4/Meshes/SK_Mannequin.SK_Mannequin")
  (Transformation|SetRelativeLocation (Variables|Character|GetMesh) "0.000000,0.000000,-90.000000" false false))

(event Custom|Transform%20to%20monster
  ;[1 1 1] Transform to monster
  (Components|SkeletalMesh|SetSkeletalMeshAsset (Variables|Character|GetMesh) "/Game/Enemy/monster/monster1.monster1")
  (Transformation|SetRelativeLocation (Variables|Character|GetMesh) "0.000000,0.000000,50.000000" false false))

(event Custom|Speak
  ;[1 1 1] Monster speak
  (if (< (Variables|Default|GetTextNumber) 3)
    _
    (else
      (Variables|Default|SetTextNumber -1)))
  (Math|Integer|IncrementInt (Variables|Default|GetTextNumber)))

(event Custom|Playgrowlsound
  (Utilities|FlowControl|DoOnce false :!label _label
    (:Completed
      (Audio|PlaySoundatLocation (Variables|Default|GetAudio) (Transformation|GetActorLocation self) "0, 0, 0" 1.0 1.0 0.0 0 0 0 0)
      (Utilities|FlowControl|Delay 4.0)
      (goto _label Reset))))

(event EventBeginPlay
  (Collision|SetCollisionEnabled (Variables|Default|GetCatchZone) "NoCollision")
  (CallFunction|TPCheck)
  (Components|Timeline|SetPlayRate (Variables|Character|GetMesh) 3.0))

(fn ConstructionScript)